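; BP_SpawnerManager populates a level at BeginPlay with doors, indoor decor, a security alarm and valuables placed on typed spawn-marker actors.
; Each step feeds a pool to SpawnWeightedElements, which picks classes by weighted random and fills random markers up to an optional cap.
; An occupied-marker list prevents reuse by re-rolling on collisions.
; Outdoor decor, traps, NPCs and device linking are empty stubs.
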(event `self.ReceiveBeginPlay`
  (`self.SpawnDoors` "/Game/MarianoArguello/Blueprints/SpawnMarkers/BP_SpawnMarker_Door.BP_SpawnMarker_Door_C")
  (`self.SpawnIndoorDecor` "/Game/MarianoArguello/Blueprints/SpawnMarkers/BP_SpawnMarker_Container.BP_SpawnMarker_Container_C" "/Game/MarianoArguello/Blueprints/SpawnMarkers/BP_SpawnMarker_Seat.BP_SpawnMarker_Seat_C" "/Game/MarianoArguello/Blueprints/SpawnMarkers/BP_SpawnMarker_Table.BP_SpawnMarker_Table_C" "/Game/MarianoArguello/Blueprints/SpawnMarkers/BP_SpawnMarker_Decor_Small.BP_SpawnMarker_Decor_Small_C")
  (`self.SpawnSecurityAlarm` "/Game/MarianoArguello/Blueprints/SpawnMarkers/BP_SpawnMarker_Alarm.BP_SpawnMarker_Alarm_C")
  (`self.SpawnValuables` "/Game/MarianoArguello/Blueprints/SpawnMarkers/BP_SpawnMarker_Valuable.BP_SpawnMarker_Valuable_C")
  (`self.SpawnOutdoorDecor` null)
  (`self.SpawnTraps` null)
  (`self.SpawnNPCs` null)
  (`self.LinkInteractableDevices`))

(fn `GetWeightedElement`
  (params (ElementList :type "Array of /Game/MarianoArguello/Blueprints/S_WeightedElement Structure"))
  (returns (PickedElement :type "/Game/MarianoArguello/Blueprints/S_WeightedElement Structure"))
  (locals (TotalWeight :type Integer) (AddedWeight :type Integer) (GeneratedWeight :type Integer) (ChosenElement :type "/Game/MarianoArguello/Blueprints/S_WeightedElement Structure"))
  (for _array_element ElementList
    (bind _output_get (set `local.TotalWeight` (+ (`.Weight_5_897301F04996CA0F2BCBE39388BD4883` (break `/Game/MarianoArguello/Blueprints/S_WeightedElement` _array_element)) (`local.TotalWeight`)))))
  (bind _returnvalue (`KismetMathLibrary.RandomIntegerInRange` 0 _output_get))
  (set `local.GeneratedWeight` _returnvalue)
  (for _array_element_2 ElementList
    (bind _output_get_2 (set `local.AddedWeight` (+ (`.Weight_5_897301F04996CA0F2BCBE39388BD4883` (break `/Game/MarianoArguello/Blueprints/S_WeightedElement` _array_element_2)) (`local.AddedWeight`))))
    (if (<= (`local.GeneratedWeight`) _output_get_2)
      (set `local.ChosenElement` _array_element_2)
      (`|ExecutionSequence`
        (:`then_0`
          (break))
        (:`then_1`
          (return (`local.ChosenElement`)))))))

(fn `LinkInteractableDevices`)

(fn `SpawnDoors`
  (params (DoorMarker :type "/Game/MarianoArguello/Blueprints/BP_SpawnMarker Class Reference"))
  (`self.SpawnWeightedElements` DoorMarker -1 (`self.DoorPool`)))

(fn `SpawnIndoorDecor`
  (params (`Container Marker` :type "/Game/MarianoArguello/Blueprints/BP_SpawnMarker Class Reference") (`Seat Marker` :type "/Game/MarianoArguello/Blueprints/BP_SpawnMarker Class Reference") (`Table Marker` :type "/Game/MarianoArguello/Blueprints/BP_SpawnMarker Class Reference") (`Small Decor Marker` :type "/Game/MarianoArguello/Blueprints/BP_SpawnMarker Class Reference"))
  (`|ExecutionSequence`
    (:`then_0`
      ; Spawn Step: Containers
      (`self.SpawnWeightedElements` `Container Marker` -1 (`self.ContainerPool`)))
    (:`then_1`
      ; Spawn Step: Seats
      (`self.SpawnWeightedElements` `Seat Marker` -1 (`self.SeatPool`)))
    (:`then_2`
      ; Spawn Step: Tables
      (`self.SpawnWeightedElements` `Table Marker` -1 (`self.TablePool`)))
    (:`then_3`
      ; Spawn Step: Small Decorators
      (`self.SpawnWeightedElements` `Small Decor Marker` -1 (`self.SmallDecorPool`)))))

(fn `SpawnNPCs`
  (params (`NPC Marker` :type "/Game/MarianoArguello/Blueprints/BP_SpawnMarker Class Reference")))

(fn `SpawnOutdoorDecor`
  (params (`Decor Marker` :type "/Game/MarianoArguello/Blueprints/BP_SpawnMarker Class Reference")))

(fn `SpawnSecurityAlarm`
  (params (`Alarm Marker` :type "/Game/MarianoArguello/Blueprints/BP_SpawnMarker Class Reference"))
  (`self.SpawnWeightedElements` `Alarm Marker` 1 (`|MakeArray` (`self.SecurityAlarm`))))

(fn `SpawnTraps`
  (params (`Trap Marker` :type "/Game/MarianoArguello/Blueprints/BP_SpawnMarker Class Reference")))

(fn `SpawnValuables`
  (params (`Item Marker` :type "/Game/MarianoArguello/Blueprints/BP_SpawnMarker Class Reference"))
  (`self.SpawnWeightedElements` `Item Marker` (`KismetMathLibrary.RandomIntegerInRange` (`self.MinItems`) (`self.MaxItems`)) (`self.ItemPool`)))

(fn `SpawnWeightedElements`
  (params (MarkerType :type "/Game/MarianoArguello/Blueprints/BP_SpawnMarker Class Reference") (MaxSpawns :type Integer) (Elements :type "Array of /Game/MarianoArguello/Blueprints/S_WeightedElement Structure"))
  (returns (InstancedActors :type "Array of Actor Object Reference"))
  (locals (AvaiableMarkers :type "Array of /Game/MarianoArguello/Blueprints/BP_SpawnMarker Object Reference") (OccupiedMarkers :type "Array of /Game/MarianoArguello/Blueprints/BP_SpawnMarker Object Reference") (ChosenClass :type "Actor Class Reference") (SpawnCounter :type Integer) (SpawnedActors :type "Array of Actor Object Reference") (ElementList :type "Array of /Game/MarianoArguello/Blueprints/S_WeightedElement Structure"))
  (set `local.ElementList` Elements)
  (bind _outactors (`GameplayStatics.GetAllActorsOfClass` MarkerType))
  (bind _output_get (set `local.AvaiableMarkers` _outactors))
  (if (`KismetArrayLibrary.Array_IsNotEmpty` _output_get)
    (while (and (< (`local.SpawnCounter`) (`KismetArrayLibrary.Array_Length` (`local.AvaiableMarkers`))) (or (< (`local.SpawnCounter`) MaxSpawns) (<= MaxSpawns -1)))
      (bind _pickedelement (`self.GetWeightedElement` (`local.ElementList`)))
      (set `local.ChosenClass` (`.Class_4_A596D0FE426B333B3DC6D8A97603CF5C` (break `/Game/MarianoArguello/Blueprints/S_WeightedElement` _pickedelement)))
      (bind _outitem (`KismetArrayLibrary.Array_Random` (`local.AvaiableMarkers`) :!label _label))
      (if (`KismetArrayLibrary.Array_Contains` (`local.OccupiedMarkers`) _outitem)
        (`KismetSystemLibrary.PrintString` "Detected an occupied marker. Skipping to next iteration")
        (goto _label)
        (else
          (`KismetArrayLibrary.Array_Add` (`local.OccupiedMarkers`) _outitem)
          (bind _returnvalue (`|SpawnActorFromClass` (`local.ChosenClass`) (`self.GetTransform` _outitem) "AdjustIfPossibleButAlwaysSpawn" "MultiplyWithRoot" self null))
          (`/Engine/EditorBlueprintResources/StandardMacros.IncrementInt` (`local.SpawnCounter`)
            (:`  `
              (`KismetArrayLibrary.Array_Add` (`local.SpawnedActors`) _returnvalue))))))
    (return (`local.SpawnedActors`))))

(fn `UserConstructionScript`)