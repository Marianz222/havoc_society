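; Interactive button level object that broadcasts press start and end events when interacted with and exposes whether it is linked.
; Interact plays a timeline whose every update calls Activate, which re-broadcasts the start event, prints a debug message, sets Active and sets the button mesh's relative location.
; On finish it clears Active, broadcasts the end event and resets the timeline time.
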(event `/Game/MarianoArguello/BlueprintInterfaces/BPI_Interactable.Interact`
  (params (Owner :type "Actor Object Reference"))
  (bind (_direction _floattrack) (`Timeline|Interaction Timeline` :!label _label)
    (:`Update`
      (`self.Activate` _floattrack))
    (:`Finished`
      (set `self.Active` false)
      (`self.OnButtonPressedEnd`)
      (goto _label :!via `SetNewTime`))))

(fn `Activate`
  (params (Time :type "Float (double-precision)"))
  (locals (PushDistance :type "Float (double-precision)" :default 50.0))
  (`|ExecutionSequence`
    (:`then_0`
      (`self.OnButtonPressedStart`)
      (`KismetSystemLibrary.PrintString` "Boton presionado"))
    (:`then_1`
      (set `self.Active` true)
      (`SceneComponent.K2_SetRelativeLocation` (`self.Button`) (0.0 0.0 0.0) false false))))

(fn `IsLinked`
  (returns (Linked :type Boolean))
  (return (`self.Linked`)))

(fn `UserConstructionScript`)