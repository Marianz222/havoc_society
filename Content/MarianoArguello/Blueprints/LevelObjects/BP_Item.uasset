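; BP_Item is a collectable valuable that rolls a random worth between MinWorth and MaxWorth at BeginPlay.
; Interact runs Collect, which asks the collector through message calls whether its inventory is empty, then hands itself over as the held item and destroys itself.
; GetItemValue exposes the worth.
; The debug print re-evaluates the random node, so its logged value can differ from the stored one.
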(event `self.ReceiveBeginPlay`
  (`self.SetInitialValue`))

(event `/Game/MarianoArguello/BlueprintInterfaces/BPI_Interactable.Interact`
  (params (Owner :type "Actor Object Reference"))
  (`/Game/MarianoArguello/BlueprintInterfaces/BPI_Collectable.Collect` Owner))

(fn `Collect`
  (params (Collector :type "Actor Object Reference"))
  (returns (CanCollect :type Boolean))
  (locals (Collectable :type Boolean))
  (`KismetSystemLibrary.PrintString` (`KismetStringLibrary.Concat_StrStr` "Recolector: " (`KismetSystemLibrary.GetDisplayName` Collector)))
  (bind _emptyinventory (message `/Game/MarianoArguello/BlueprintInterfaces/BPI_Player.IsInventoryEmpty` Collector))
  (if _emptyinventory
    (set `local.Collectable` true)
    (message `/Game/MarianoArguello/BlueprintInterfaces/BPI_Player.SetHeldItem` Collector self)
    (`self.K2_DestroyActor`)
    (return (`local.Collectable`))
    (else
      (set `local.Collectable` false))))

(fn `GetItemValue`
  (returns (Value :type Integer))
  (return (`self.Value`)))

(fn `SetInitialValue`
  (bind _returnvalue (`KismetMathLibrary.RandomIntegerInRange` (`self.MinWorth`) (`self.MaxWorth`)))
  (set `self.Value` _returnvalue)
  (`KismetSystemLibrary.PrintString` (`KismetStringLibrary.Concat_StrStr` "Valuable: " (`KismetSystemLibrary.GetDisplayName` self) " was created with value: " (`KismetStringLibrary.Conv_IntToString` _returnvalue))))

(fn `UserConstructionScript`)