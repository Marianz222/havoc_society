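; CCTV trap for levels: a security camera that sweeps back and forth and detects targetable actors.
; Every Tick, a box trace from the camera body looks for a BPI_Targetable actor and calls OnTargetedMessage on it.
; While a target is held, a point light shows and the scan timeline stops.
; Otherwise the light hides and the timeline resumes, scaling its float track by MaxAngle into camera yaw.
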(event `self.ReceiveBeginPlay`)

(event `self.ReceiveTick`
  (params (DeltaSeconds :type "Float (single-precision)"))
  (bind _pointlight (`self.PointLight`))
  (bind (_hastarget _targetedactor) (`self.TrackTarget`))
  (set `self.CurrentTarget` _targetedactor)
  (if _hastarget
    (`SceneComponent.SetVisibility` _pointlight true false)
    (bind (_direction _floattrack) (`Timeline|Scan Environment Timeline` :!via `Stop` :!label _label)
      (:`Update`
        (`self.ScanEnvironment` _floattrack)
        (if (`self.Debugging`)
          (`KismetSystemLibrary.PrintString` (`KismetStringLibrary.Concat_StrStr` "Timeline value: " (`KismetStringLibrary.Conv_DoubleToString` _floattrack))))))
    (else
      (`SceneComponent.SetVisibility` _pointlight false false)
      (goto _label))))

(fn `ScanEnvironment`
  (params (Time :type "Float (double-precision)"))
  (locals (FacingRight :type Boolean))
  (`SceneComponent.K2_SetRelativeRotation` (`self.CameraBody`) (`KismetMathLibrary.MakeRotator` 0.0 0.0 (* Time (`self.MaxAngle`))) false false))

(fn `TrackTarget`
  (returns (HasTarget :type Boolean) (TargetedActor :type "Actor Object Reference"))
  (bind _camerabody (`self.CameraBody`))
  (bind _returnvalue (`SceneComponent.K2_GetComponentLocation` _camerabody))
  (bind _outhit (`KismetSystemLibrary.BoxTraceSingle` :`Start` _returnvalue :`End` (+ (* (`SceneComponent.GetForwardVector` _camerabody) (`self.MaxDetectionRange`)) _returnvalue) :`HalfSize` (15.0 30.0 25.0) :`TraceChannel` "TraceTypeQuery4" :`DrawDebugType` "ForOneFrame"))
  (`|ExecutionSequence`
    (:`then_0`
      (if (`self.Debugging`)
        (bind (_bblockinghit _binitialoverlap _time _distance _location _impactpoint _normal _impactnormal _physmat _hitactor) (`GameplayStatics.BreakHitResult` _outhit))
        (`KismetSystemLibrary.PrintString` (`KismetStringLibrary.Concat_StrStr` "Object hit: " (`KismetSystemLibrary.GetDisplayName` _hitactor)))))
    (:`then_1`
      (if (`KismetSystemLibrary.DoesImplementInterface` _hitactor "/Game/MarianoArguello/BlueprintInterfaces/BPI_Targetable.BPI_Targetable_C")
        (set `self.IsTargeting` true)
        (message `/Game/MarianoArguello/BlueprintInterfaces/BPI_Targetable.OnTargeted` _hitactor)
        (else
          (set `self.IsTargeting` false)))
      (return (`self.IsTargeting`) _hitactor))))

(fn `UserConstructionScript`)