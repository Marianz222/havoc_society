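; BP_Door is an interactable hinged door that prints a Spanish "door is blocked" message when locked.
; When unlocked, Interact plays OpeningTimeline, whose updates check Opened each time and pass the float track to Close or Open.
; Open sets Opened immediately, then derives the Hinge's relative rotation from that value, OpeningAngle and the actor's rotation.
; IsLocked and IsOpen expose the state; Close's body is absent here.
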(event `/Game/MarianoArguello/BlueprintInterfaces/BPI_Interactable.Interact`
  (params (Owner :type "Actor Object Reference"))
  (if (`self.Locked`)
    (`KismetSystemLibrary.PrintString` "La puerta esta bloqueada")
    (else
      (bind (_direction _floattrack) (`Timeline|Opening Timeline`)
        (:`Update`
          (if (`self.Opened`)
            (`self.Close` _floattrack)
            (else
              (`self.Open` _floattrack))))))))

(fn `IsLocked`
  (returns (Locked :type Boolean))
  (return (`self.Locked`)))

(fn `IsOpen`
  (returns (Opened :type Boolean))
  (return (`self.Opened`)))

(fn `Open`
  (params (AnimationTime :type "Float (double-precision)"))
  (bind (_returnvalue_location _returnvalue_rotation) (`KismetMathLibrary.BreakTransform` (`self.GetTransform`)))
  (set `self.Opened` true)
  (`SceneComponent.K2_SetRelativeRotation` (`self.Hinge`) (`KismetMathLibrary.Conv_VectorToRotator` (`KismetMathLibrary.GreaterGreater_VectorRotator` (`KismetMathLibrary.MakeVector` (* AnimationTime (`self.OpeningAngle`))) _returnvalue_rotation)) false false)
  (return))

(fn `UserConstructionScript`)