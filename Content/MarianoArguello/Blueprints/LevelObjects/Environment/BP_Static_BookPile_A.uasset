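; Environment book pile prop that varies its appearance at runtime by randomizing materials.
; On BeginPlay, RandomizeColors gives each of the Outside1, Outside2 and Outside3 components an independent random pick from AvaiableMaterials on material slot 0.
; The construction script is empty, so this code applies no randomization in the editor.
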(event `self.ReceiveBeginPlay`
  (`self.RandomizeColors`))

(fn `RandomizeColors`
  (`PrimitiveComponent.SetMaterial` (`self.Outside1`) 0 (`KismetArrayLibrary.Array_Random` (`self.AvaiableMaterials`)))
  (`PrimitiveComponent.SetMaterial` (`self.Outside2`) 0 (`KismetArrayLibrary.Array_Random` (`self.AvaiableMaterials`)))
  (`PrimitiveComponent.SetMaterial` (`self.Outside3`) 0 (`KismetArrayLibrary.Array_Random` (`self.AvaiableMaterials`))))

(fn `UserConstructionScript`)