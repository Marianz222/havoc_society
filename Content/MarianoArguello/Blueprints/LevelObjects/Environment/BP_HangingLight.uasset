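; BP_HangingLight is an environment level object for a hanging light with a spot light and a point light component.
; On BeginPlay, SetInitialState copies StartActivated into Active, then branches to activate or deactivate both lights.
; The branch condition is a constant true rather than that flag, so both lights are always activated and the deactivate path never runs.
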(event `self.ReceiveBeginPlay`
  (`self.SetInitialState`))

(fn `SetInitialState`
  (bind _pointlight (`self.PointLight`))
  (bind _spotlight (`self.SpotLight`))
  (set `self.Active` (`self.StartActivated`))
  (if true
    (`|ExecutionSequence`
      (:`then_0`
        (`ActorComponent.Activate` _spotlight false))
      (:`then_1`
        (`ActorComponent.Activate` _pointlight false)))
    (else
      (`|ExecutionSequence`
        (:`then_0`
          (`ActorComponent.Deactivate` _spotlight))
        (:`then_1`
          (`ActorComponent.Deactivate` _pointlight))))))

(fn `UserConstructionScript`)