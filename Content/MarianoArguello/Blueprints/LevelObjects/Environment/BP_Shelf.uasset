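; BP_Shelf is an environment level object that randomly places item spawners on itself when play begins.
; SpawnerSetup gathers the child components of Spawners as candidate points and spawns BP_Spawner_Item actors at random ones until MaxLootSpawners is reached.
; Used indexes are tracked and duplicates re-rolled, with no guard for a maximum exceeding the available points, which would leave the loop unable to finish.
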(event `self.ReceiveBeginPlay`
  (`self.SpawnerSetup`))

(fn `SpawnerSetup`
  (locals (SpawnerList :type "Array of SceneComponent Object Reference") (UsedIndexes :type "Array of Integer"))
  (bind _output_get (set `local.SpawnerList` (`SceneComponent.GetChildrenComponents` (`self.Spawners`) false)))
  (if (and (`KismetArrayLibrary.Array_IsNotEmpty` _output_get) (> (`self.MaxLootSpawners`) 0))
    (while (< (`self.LootSpawnerCounter`) (`self.MaxLootSpawners`))
      (bind (_outitem _outindex) (`KismetArrayLibrary.Array_Random` (`local.SpawnerList`)))
      (if (`KismetArrayLibrary.Array_Contains` (`local.UsedIndexes`) _outindex)
        (`KismetSystemLibrary.PrintString` "Chosen index was already taken. Retrying...")
        (else
          (`KismetArrayLibrary.Array_Add` (`local.UsedIndexes`) _outindex)
          (`|SpawnActorFromClass` "/Game/MarianoArguello/Blueprints/Spawners/InitializationBased/BP_Spawner_Item.BP_Spawner_Item_C" (`KismetMathLibrary.MakeTransform` (`SceneComponent.K2_GetComponentLocation` _outitem)) "AdjustIfPossibleButAlwaysSpawn" "MultiplyWithRoot" null null)
          (`/Engine/EditorBlueprintResources/StandardMacros.IncrementInt` (`self.LootSpawnerCounter`)))))
    (`KismetSystemLibrary.PrintString` (`KismetStringLibrary.Concat_StrStr` "Completed spawner initialization for: " (`KismetSystemLibrary.GetDisplayName` self)))))

(fn `UserConstructionScript`)