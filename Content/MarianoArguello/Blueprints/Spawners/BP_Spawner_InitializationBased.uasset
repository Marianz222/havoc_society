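; A spawner actor that places one randomly chosen actor at its own transform when play begins.
; On BeginPlay, Spawn picks a random class from the PossibleActors list, spawns it with the spawner as owner and stores the result in SpawnedInstance.
; It then sets FinishedSpawning and hides itself in game.
; An empty list prints a failure message naming the spawner instead.
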(event `self.ReceiveBeginPlay`
  (`self.Spawn`))

(fn `Spawn`
  (bind _possibleactors (`self.PossibleActors`))
  (if (`KismetArrayLibrary.Array_IsNotEmpty` _possibleactors)
    (bind _returnvalue (`|SpawnActorFromClass` (`KismetArrayLibrary.Array_Random` _possibleactors) (`self.GetTransform`) "Undefined" "MultiplyWithRoot" self null))
    (set `self.SpawnedInstance` _returnvalue)
    (bind _output_get (set `self.FinishedSpawning` true))
    (`self.SetActorHiddenInGame` _output_get)
    (else
      (`KismetSystemLibrary.PrintString` (`KismetStringLibrary.Concat_StrStr` "Spawning on object: " (`KismetSystemLibrary.GetDisplayName` self) " failed. The \"PossibleActors\" list is empty")))))

(fn `UserConstructionScript`)